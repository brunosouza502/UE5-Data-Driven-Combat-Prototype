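; Sword light attack ability that deals melee damage to whatever the owner's sword hits.
; Most lifecycle functions only defer to the parent ability class, and DoMelee is empty.
; ExecuteHit calls the parent, then sphere-traces on the Visibility channel between two sword mesh sockets.
; A blocking hit plays an impact sound and applies the damage value from the ability Definition.
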(fn Activate
  (|CallParentFunction))

(fn DoMelee)

(fn Init
  (params (InOwnerActor :type BP%20Player%20Object%20Reference) (InDefinition :type DA%20Ability%20Definition%20Object%20Reference))
  (|CallParentFunction InOwnerActor InDefinition))

(fn CanActivate
  (bind (_isactive _definition) (|CallParentFunction))
  (return _isactive _definition))

(fn End
  (|CallParentFunction))

(fn ExecuteHit
  (bind _owneractor (Variables|Default|GetOwnerActor))
  (bind _sword (Variables|/Game/ProjectSword/Player/BP_Player.BP_Player_C|GetSword _owneractor))
  (bind _swordmesh (Variables|/Game/ProjectSword/Player/Sword/BP_Sword.BP_Sword_C|GetSwordMesh _sword))
  (|CallParentFunction)
  (bind _outhit (Collision|SphereTraceByChannel (Variables|Default|GetOwnerActor) (Transformation|GetSocketLocation _swordmesh "HitB") (Transformation|GetSocketLocation _swordmesh "HitA") 1e+01 "TraceTypeQuery1" false 0 "None"))
  (if (.bBlockingHit (Collision|BreakHitResult _outhit))
    (Audio|PlaySoundatLocation (Variables|Default|GetOwnerActor) "/Game/ProjectSword/Demo/Sounds/SC_Hit.SC_Hit" (.ImpactPoint (Collision|BreakHitResult _outhit)) "0, 0, 0" 1.0 1.0 0.0 0 0 0 0)
    (Game|Damage|ApplyDamage (.HitActor (Collision|BreakHitResult _outhit)) (Variables|/Game/ProjectSword/Data/Ability/DA_Ability_Definition.DA_Ability_Definition_C|GetDamage (Variables|Default|GetDefinition)) 0 0)))