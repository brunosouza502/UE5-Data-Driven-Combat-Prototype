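; Blueprint ability component for BP_Player that creates, activates and ends the player's montage-driven abilities.
; On BeginPlay it constructs and initializes an ability object from each DA_Ability_Definition, mapped by AbilityID.
; TryActivateAbility looks up the ID, checks CanActivate, then activates the ability and plays its montage.
; Montage completion or interruption ends it and resets combo and trace, while AnimNotify hits route to CurrentActiveAbility.ExecuteHit.
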(event Custom|CommitMontage
  (bind _ownercharacter (Variables|Default|GetOwnerCharacter))
  ;[0.15 0.15 0.15 0.5] Evento para garantir xecução e utilizar Completed para atualizar estado
  (Animation|Montage|PlayMontage (Variables|/Script/Engine.Character|GetMesh (Variables|Default|GetOwnerCharacter)) (Variables|/Game/ProjectSword/Data/Ability/DA_Ability_Definition.DA_Ability_Definition_C|GetMontage (Variables|/Game/ProjectSword/Data/Ability/BP_AbilityBase.BP_AbilityBase_C|GetDefinition (Variables|Default|GetAbilityDef)))
    (:OnCompleted
      _)
    (:OnInterrupted
      _))
  ;;[0.15 0.15 0.15 0.5] Resetar habildade
  (Default|End (Variables|Default|GetAbilityDef))
  ;;[0.15 0.15 0.15 0.5] Evita congelar o ataque básico, caso o player tenha executado a habilidade no meio de um combo
  (Default|ResetCombo _ownercharacter)
  (Default|ResetTrace _ownercharacter))

(event EventBeginPlay
  (CallFunction|InitializeAbilities))

(event EventTick
  (params (DeltaSeconds :type Float%20%28single-precision%29)))

(fn InitializeAbilities
  ;[0.15 0.15 0.15 0.5] Inicializa habilidades
  (for _array_element (Variables|Default|GetAbilityDefinitions)
    ;;[0.15 0.15 0.15 0.5] DA_Ability_Definition
    (bind _output_get (Variables|Default|SetDef _array_element))
    (Utilities|IsValid _output_get
      (:Is%20Valid
        ;;[0.15 0.15 0.15 0.5] Selecionado a classe com base na instância
        (bind _returnvalue (Game|ConstructObjectfromClass (Variables|/Game/ProjectSword/Data/Ability/DA_Ability_Definition.DA_Ability_Definition_C|GetAbilityClass (Variables|Default|GetDef))))
        ;;[0.15 0.15 0.15 0.5] BP_AbilityBase
        (bind _output_get_2 (Variables|Default|SetAbility _returnvalue))
        ;;[0.15 0.15 0.15 0.5] Dono da classe
        (bind _asbp_player (Utilities|Casting|CastToBP_Player (Components|GetOwner)))
        (bind _output_get_3 (Variables|Default|SetOwnerCharacter _asbp_player))
        (Default|Init _output_get_2 _output_get_3 (Variables|Default|GetDef))
        (Utilities|Map|Add (Variables|Default|GetAbilityInstances) (Variables|/Game/ProjectSword/Data/Ability/DA_Ability_Definition.DA_Ability_Definition_C|GetAbility_ID (Variables|Default|GetDef)) _output_get_2))
      (:Is%20Not%20Valid
        (Development|PrintString "Not Valid DA_Ability_Definition")))))

(fn TryActivateAbility
  (params (AbilityId :type Name))
  (bind _abilityinstances (Variables|Default|GetAbilityInstances))
  (bind (_value _returnvalue) (Utilities|Map|Find _abilityinstances AbilityId))
  (Variables|Default|SetCurrentActiveAbility (Variables|Default|GetAbility))
  (if _returnvalue
    (Utilities|IsValid _value
      (:Is%20Valid
        (Variables|Default|SetAbilityDef _value)
        (bind _isactive (Default|CanActivate (Variables|Default|GetAbilityDef)))
        (if (not _isactive)
          (CallFunction|PlayAbilityMontage))))))

(fn PlayAbilityMontage
  ;[0.15 0.15 0.15 0.5] Habilidade Ativa
  (Default|Activate (Variables|Default|GetAbilityDef))
  (CallFunction|CommitMontage))

(fn NotifyCurrentAbilityHit
  ;[0.15 0.15 0.15 0.5] Called in AnimNotify - then in AnimNotify
  (bind _currentactiveability (Variables|Default|GetCurrentActiveAbility)
    (:then
      (Default|ExecuteHit _currentactiveability))
    (:else)))