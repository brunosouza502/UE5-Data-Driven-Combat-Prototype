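; BP_SwordComponent is a player component that spawns and removes the sword held by its owning BP_Player.
; BeginPlay caches the owner, then EquipSword spawns a SwordBase at the SwordHand socket and initializes it from SwordDef.
; It caches the sword's mesh and damage, then snaps that static mesh, rather than the actor, to the socket.
; Clear destroys the sword actor; its IsDead check is disconnected, and debug prints remain.
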(event EventBeginPlay
  (bind _asbp_player (Utilities|Casting|CastToBP_Player (Components|GetOwner)))
  (Variables|Default|SetAs%20BP%20Player _asbp_player))

(event EventTick
  (params (DeltaSeconds :type Float%20%28single-precision%29)))

(fn EquipSword
  (bind _returnvalue (Game|SpawnActorfromClass "/Script/ProjectSwordRepo.SwordBase" (Transformation|GetSocketTransform (Variables|/Script/Engine.Character|GetMesh (Variables|Default|GetAs%20BP%20Player)) "SwordHand" "RTS_World") "Undefined" "MultiplyWithRoot" 0 0))
  (bind _output_get (Variables|Default|SetSwordActorRef _returnvalue))
  (Utilities|IsValid _output_get
    (:Is%20Valid
      (Development|PrintString (Utilities|GetDisplayName _output_get))
      (Class|SwordBase|Init _output_get (Variables|Default|GetSwordDef) (Variables|Default|GetAs%20BP%20Player))
      (Variables|Default|SetSword%20Static%20Mesh (Variables|/Script/ProjectSwordRepo.SwordBase|GetSwordStaticMesh (Variables|Default|GetSwordActorRef)))
      (Variables|Default|SetDamage (Variables|/Script/ProjectSwordRepo.SwordDefinition|GetDamage (Variables|Default|GetSwordDef)))
      (Transformation|AttachComponentToComponent (Variables|/Script/ProjectSwordRepo.SwordBase|GetSwordStaticMesh (Variables|Default|GetSwordActorRef)) (Variables|/Script/Engine.Character|GetMesh (Variables|Default|GetAs%20BP%20Player)) "SwordHand" "SnapToTarget" "SnapToTarget" "SnapToTarget" true)
      (Development|PrintString (Utilities|GetDisplayName (Variables|Default|GetSwordActorRef))))))

(fn Clear
  (Development|PrintString "Entrou em Clear")
  (bind _swordactorref (Variables|Default|GetSwordActorRef)
    (:then
      (Actor|DestroyActor _swordactorref)
      (bind _output_get (Variables|Default|SetSwordActorRef 0))
      (Development|PrintString "SwordActorRef")
      (Development|PrintString (Utilities|GetDisplayName _output_get)))
    (:else)))