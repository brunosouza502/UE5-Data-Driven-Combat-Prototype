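; BP_AbilityBase is a base class for abilities, holding an owner actor and an ability definition passed in through Init.
; Activate sets an IsActive flag and prints it as debug text, and End clears it.
; CanActivate returns the raw IsActive flag, not its inverse.
; ExecuteHit is an empty function, and no hit logic exists at this level.
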(fn Init
  (params (InOwnerActor :type BP%20Player%20Object%20Reference) (InDefinition :type DA%20Ability%20Definition%20Object%20Reference))
  (Variables|Default|SetOwnerActor InOwnerActor)
  (Variables|Default|SetDefinition InDefinition))

(fn CanActivate
  (return (Variables|Default|GetbIsActive) 0))

(fn Activate
  (bind _output_get (Variables|Default|SetbIsActive true))
  (Development|PrintString 0 (Utilities|String|ToString(Boolean) _output_get) true true "(R=1.000000,G=0.000000,B=0.000000,A=1.000000)"))

(fn End
  (Variables|Default|SetbIsActive false))

(fn ExecuteHit)