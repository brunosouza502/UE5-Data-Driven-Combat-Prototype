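; Actor component on BP_Player that bridges Blueprint to the C++ light attack ability.
; ActivateLightAttackCPP calls EnsureCppAbilityInitialized, which constructs a fresh ability object on every call and initializes it with its data asset and the owner cached at BeginPlay, then activates it.
; OnHitFrame forwards to that instance's ExecuteHit while it is active.
; Debug prints trace each stage, and leftover EventGraph initialization nodes never run.
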(event EventBeginPlay
  (bind _asbp_player (Utilities|Casting|CastToBP_Player (Components|GetOwner)))
  (Variables|Default|SetOwnerCharacter _asbp_player))

(fn ActivateLightAttackCPP
  (bind _lightattackcppinstance (Variables|Default|GetLightAttackCppInstance))
  (Development|PrintString "ASC Called")
  (CallFunction|EnsureCppAbilityInitialized)
  (Variables|Default|GetLightAttackCppInstance
    (:then
      (Class|AbilityBaseCpp|DebugPing _lightattackcppinstance)
      (Class|AbilityBaseCpp|ActivateAbility _lightattackcppinstance))
    (:else)))

(fn EnsureCppAbilityInitialized
  (bind _returnvalue (Game|ConstructObjectfromClass (Variables|Default|GetLightAttackCppClass)))
  (Development|PrintString "Constucted")
  (bind _output_get (Variables|Default|SetTempObj _returnvalue))
  (bind _aslight_attack_ability_cpp (Utilities|Casting|CastToLightAttackAbilityCpp _output_get))
  (Development|PrintString "Cast Ok")
  (bind _output_get_2 (Variables|Default|SetTempAbility _aslight_attack_ability_cpp))
  (bind _output_get_3 (Variables|Default|SetLightAttackCppInstance _output_get_2))
  (Development|PrintString (Utilities|GetClassDisplayName (Utilities|GetClass _output_get_3)) true true "(R=1.000000,G=0.000000,B=0.000000,A=1.000000)")
  (Development|PrintString (Utilities|GetDisplayName (Variables|Default|GetOwnerCharacter)))
  (Class|AbilityBaseCpp|Init _output_get_3 (Variables|Default|GetDA_LightAttack_CPP) (Variables|Default|GetOwnerCharacter))
  (Development|PrintString "Init ok"))

(fn OnHitFrame
  (bind _lightattackcppinstance (Variables|Default|GetLightAttackCppInstance)
    (:then
      (if (Variables|/Script/ProjectSwordRepo.AbilityBaseCpp|GetbIsActive _lightattackcppinstance)
        (Development|PrintString (Utilities|GetDisplayName _lightattackcppinstance) true true "(R=1.000000,G=0.000000,B=0.000000,A=1.000000)" 5.0)
        (Class|AbilityBaseCpp|ExecuteHit _lightattackcppinstance)))
    (:else
      (Development|PrintString "Invalid"))))